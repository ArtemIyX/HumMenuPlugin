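; Server filter object for a boolean option in the server filters, represented in the UI by a checkbox.
; It extends a parent filter by creating a checkbox widget with the filter name, giving it a reference to itself and binding to its update event.
; On a checkbox update it fires the server filter update, then stores the checked state and broadcasts it through a bool filter update call.
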(fn GetServerFilterWidget
  (params (WorldContextObject :type Object%20Object%20Reference) (InPlayerController :type Player%20Controller%20Object%20Reference))
  (|CallParentFunction WorldContextObject InPlayerController)
  (bind _returnvalue (UserInterface|CreateWidget WorldContextObject "/HumMenuPlugin/MenuWIdgetElements/ServerMenuElements/WB_FilterCheckBoxx.WB_FilterCheckBoxx_C" InPlayerController (Variables|Default|GetFilterName)))
  (Variables|/HumMenuPlugin/MenuWIdgetElements/ServerMenuElements/WB_FilterCheckBoxx.WB_FilterCheckBoxx_C|SetSelfObject _returnvalue self)
  (EventDispatchers|BindEventtoUpdateBoolFilter _returnvalue (EventDispatchers|CreateEvent :!event OnCheckboxUpdated))
  (return _returnvalue))

(fn OnCheckboxUpdated
  (params (IsChecked :type Boolean))
  (Class|ServerFilterObject|CallUpdateServerFilter self)
  (bind _output_get (Variables|Default|SetIs%20Checked IsChecked))
  (Default|CallOnBoolFilterUpdated _output_get))