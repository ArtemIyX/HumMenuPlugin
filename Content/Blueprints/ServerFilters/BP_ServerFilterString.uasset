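; BP_ServerFilterString is a server filter Blueprint that supplies the UI widget for a string-based filter.
; GetServerFilterWidget calls its parent, then creates and returns a WB_FilterCheckBox, passing it the combo box options and a reference to the filter.
; It also binds an event to the widget's string filter update.
; An auto-generated function calls UpdateServerFilter on the filter.
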(fn GetServerFilterWidget
  (params (WorldContextObject :type Object%20Object%20Reference) (PlayerController :type Player%20Controller%20Object%20Reference))
  (|CallParentFunction WorldContextObject PlayerController)
  (bind _returnvalue (UserInterface|CreateWidget WorldContextObject "/HumMenuPlugin/MenuWIdgetElements/ServerMenuElements/WB_FilterCheckBox.WB_FilterCheckBox_C" PlayerController (Variables|Default|GetOptionsComboBox)))
  (Variables|/HumMenuPlugin/MenuWIdgetElements/ServerMenuElements/WB_FilterCheckBox.WB_FilterCheckBox_C|SetSelfObject _returnvalue self)
  (EventDispatchers|BindEventtoUpdatelStringFilter _returnvalue (EventDispatchers|CreateEvent :!event BPServerFilterStringAutoGenFunc))
  (return _returnvalue))

(fn BPServerFilterStringAutoGenFunc
  (Class|ServerFilterObject|CallUpdateServerFilter self))