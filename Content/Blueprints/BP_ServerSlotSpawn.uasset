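; BP_ServerSlotSpawn is a server entry object that creates the UI widgets for a server slot and its info panel.
; GetServerSlotWidget overrides the parent to create a WB_ServerSlotButton for the given player controller, passing in its own ping, name, country and a self reference.
; GetServerInfoWidget likewise calls the parent, then creates and returns a WB_ServerInfo widget without passing it any server data.
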(fn GetServerSlotWidget
  (params (WorldContextObject :type Object%20Object%20Reference) (InPlayerController :type Player%20Controller%20Object%20Reference))
  (|CallParentFunction WorldContextObject InPlayerController)
  (bind _returnvalue (UserInterface|CreateWidget WorldContextObject "/HumMenuPlugin/MenuWIdgetElements/Buttons/WB_ServerSlotButton.WB_ServerSlotButton_C" InPlayerController (Variables|Default|GetPing) (Variables|Default|GetName) (Variables|Default|GetCountry) self))
  (return _returnvalue))

(fn GetServerInfoWidget
  (params (WorldContextObject :type Object%20Object%20Reference) (InPlayerController :type Player%20Controller%20Object%20Reference))
  (|CallParentFunction WorldContextObject InPlayerController)
  (bind _returnvalue (UserInterface|CreateWidget WorldContextObject "/HumMenuPlugin/MenuWIdgetElements/ServerMenuElements/WB_ServerInfo.WB_ServerInfo_C" InPlayerController))
  (return _returnvalue))