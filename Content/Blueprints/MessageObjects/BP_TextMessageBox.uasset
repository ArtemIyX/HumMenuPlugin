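; BP_TextMessageBox is a message object that shows a message box for text entry and handles the submitted text.
; It creates a WB_TextMessageBox widget, starts it with title, info and hint text plus itself, and registers it with BPC_MenuManager on the player's HUD.
; On apply, it passes the entered text to ApplyButtonEvent, then has the menu manager remove the box.
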(event EventAddMessagetoViewport
  (params (PlayerController :type Player%20Controller%20Object%20Reference))
  (bind _returnvalue (CallFunction|GetMessageBoxWidget PlayerController PlayerController))
  (Default|AddMessageBox (Actor|GetComponentbyClass (HUD|GetHUD PlayerController) "/HumMenuPlugin/BPC_MenuManager.BPC_MenuManager_C") _returnvalue self))

(fn GetMessageBoxWidget
  (params (WorldContextObject :type Object%20Object%20Reference) (InPlayerController :type Player%20Controller%20Object%20Reference))
  (|CallParentFunction WorldContextObject InPlayerController)
  (bind _returnvalue (Class|MessageBoxBase|CreateNewWidget InPlayerController "/HumMenuPlugin/MenuWIdgetElements/MessagesUI/WB_TextMessageBox.WB_TextMessageBox_C"))
  (bind _aswb_text_message_box (Utilities|Casting|CastToWB_TextMessageBox _returnvalue))
  (Default|StartWidget _aswb_text_message_box (Variables|Default|GetMessageTitleText) (Variables|Default|GetMessageInfoText) self (Variables|Default|GetHintTextBox))
  (return _returnvalue))

(fn OnApplyEvent
  (params (EnteredText :type Text) (CurrentPlayerController :type Player%20Controller%20Object%20Reference))
  (Class|TextMessageBox|ApplyButtonEvent EnteredText)
  (Default|RemoveMessageBox (Actor|GetComponentbyClass (HUD|GetHUD CurrentPlayerController) "/HumMenuPlugin/BPC_MenuManager.BPC_MenuManager_C")))