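; BP_ApplyMessageBox is a message object that builds and shows a WB_MessageBox for a player, displaying its title and info text.
; Its GetMessageBoxWidget override calls the parent, creates the widget and initializes it with the texts and itself as the owning object.
; AddMessagetoViewport gets that widget and passes it, with the object, to the BPC_MenuManager component on the player's HUD.
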(event EventAddMessagetoViewport
  (params (PlayerController :type Player%20Controller%20Object%20Reference))
  (bind _returnvalue (CallFunction|GetMessageBoxWidget PlayerController PlayerController))
  (Default|AddMessageBox (Actor|GetComponentbyClass (HUD|GetHUD PlayerController) "/HumMenuPlugin/BPC_MenuManager.BPC_MenuManager_C") _returnvalue self))

(fn GetMessageBoxWidget
  (params (WorldContextObject :type Object%20Object%20Reference) (InPlayerController :type Player%20Controller%20Object%20Reference))
  (|CallParentFunction WorldContextObject InPlayerController)
  (bind _returnvalue (Class|MessageBoxBase|CreateNewWidget InPlayerController "/HumMenuPlugin/MenuWIdgetElements/MessagesUI/WB_MessageBox.WB_MessageBox_C"))
  (bind _aswb_message_box (Utilities|Casting|CastToWB_MessageBox _returnvalue))
  (Default|StartWidget _aswb_message_box (Variables|Default|GetMessageTitleText) (Variables|Default|GetMessageInfoText) self)
  (return _returnvalue))