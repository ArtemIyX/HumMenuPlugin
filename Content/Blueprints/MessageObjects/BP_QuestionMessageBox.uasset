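; Message object for a question pop-up that shows a title and info text through the WB_QuestionMessageBox widget.
; Creates the widget for the given player controller, starts it with itself as the owning object, and registers both with the HUD's BPC_MenuManager.
; On apply, it fires ApplyButtonEvent and then has the menu manager remove the message box.
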(event EventAddMessagetoViewport
  (params (PlayerController :type Player%20Controller%20Object%20Reference))
  (bind _returnvalue (CallFunction|GetMessageBoxWidget PlayerController PlayerController))
  (Default|AddMessageBox (Actor|GetComponentbyClass (HUD|GetHUD PlayerController) "/HumMenuPlugin/BPC_MenuManager.BPC_MenuManager_C") _returnvalue self))

(fn GetMessageBoxWidget
  (params (WorldContextObject :type Object%20Object%20Reference) (InPlayerController :type Player%20Controller%20Object%20Reference))
  (|CallParentFunction WorldContextObject InPlayerController)
  (bind _returnvalue (Class|MessageBoxBase|CreateNewWidget InPlayerController "/HumMenuPlugin/MenuWIdgetElements/MessagesUI/WB_QuestionMessageBox.WB_QuestionMessageBox_C"))
  (bind _aswb_question_message_box (Utilities|Casting|CastToWB_QuestionMessageBox _returnvalue))
  (Default|StartWidget _aswb_question_message_box (Variables|Default|GetMessageTitleText) (Variables|Default|GetMessageInfoText) self)
  (return _returnvalue))

(fn OnApplyEvent
  (params (CurrentPlayerController :type Player%20Controller%20Object%20Reference))
  (Class|QuestionMessageBox|ApplyButtonEvent)
  (Default|RemoveMessageBox (Actor|GetComponentbyClass (HUD|GetHUD CurrentPlayerController) "/HumMenuPlugin/BPC_MenuManager.BPC_MenuManager_C")))