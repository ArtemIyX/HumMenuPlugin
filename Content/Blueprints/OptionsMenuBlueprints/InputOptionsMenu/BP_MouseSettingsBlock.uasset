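; Options-menu block for mouse settings in the input options menu, apparently holding test content.
; Overrides GenerateOptions, calling the parent first, then constructing option objects, appending them to OptionsArr and returning the array.
; It adds two float options, a sensitivity test and a generically named second widget, plus a byte option labelled DLSS with a preset current value.
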(fn GenerateOptions
  (params (WorldContextObject :type Object%20Object%20Reference) (InPlayerController :type Player%20Controller%20Object%20Reference))
  (|CallParentFunction WorldContextObject InPlayerController)
  (bind _returnvalue (Game|ConstructObjectfromClass WorldContextObject "/HumMenuPlugin/Blueprints/OptionsMenuBlueprints/MainObjects/BP_OptionFloat.BP_OptionFloat_C" "SensetivityTest" 0))
  (Utilities|Array|Add (LocalVariables|GetOptionsArr) _returnvalue)
  (bind _returnvalue_2 (Game|ConstructObjectfromClass "/HumMenuPlugin/Blueprints/OptionsMenuBlueprints/MainObjects/BP_OptionFloat.BP_OptionFloat_C" "Widget 2" 0))
  (Utilities|Array|Add (LocalVariables|GetOptionsArr) _returnvalue_2)
  (bind _returnvalue_3 (Game|ConstructObjectfromClass "/HumMenuPlugin/Blueprints/OptionsMenuBlueprints/MainObjects/BP_OptionByte.BP_OptionByte_C" 2 "DLSS" 0))
  (Utilities|Array|Add (LocalVariables|GetOptionsArr) _returnvalue_3)
  (return (LocalVariables|GetOptionsArr)))