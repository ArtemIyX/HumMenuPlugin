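; BP_ControlSettingsBlock is an options menu block that builds key rebinding options for the player's Enhanced Input controls.
; It registers mapping contexts from a widget properties data asset with the user settings and caches the current profile's key mappings.
; GenerateOptions creates a BP_OptionKey for each listed action's first-slot mapping.
; CanBindNewKey rejects keys already mapped, and SetNewKey remaps the first slot.
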(fn GenerateOptions
  (params (WorldContextObject :type Object%20Object%20Reference) (InPlayerController :type Player%20Controller%20Object%20Reference))
  (|CallParentFunction WorldContextObject InPlayerController)
  (Variables|Default|SetUserPlayerController InPlayerController)
  (CallFunction|RegisterMappingContexts)
  (Variables|Default|SetUserSettings (Class|EnhancedInputSubsystemInterface|GetUserSettings (PlayerController|LocalPlayerSubsystems|GetEnhancedInputLocalPlayerSubsystem InPlayerController)))
  (CallFunction|GetUserKeyMapping)
  (bind _returnvalue (Class|MenuPluginBlueprintLibrary|GetWidgetPropertiesDataAsset))
  (bind _returnvalue_2 (Utilities|LoadAssetBlocking _returnvalue))
  (bind _aswidgets_properties_data_asset (Utilities|Casting|CastToWidgetsPropertiesDataAsset _returnvalue_2))
  (for (_array_element _array_index) (Variables|/Script/HumMenuPlugin.BindingMappingsDataAsset|GetBindingMappings (Variables|/Script/HumMenuPlugin.WidgetsPropertiesDataAsset|GetBindingMappings _aswidgets_properties_data_asset))
    (for _array_element_2 (Variables|Default|GetUserKeyMapping)
      (if (and (Utilities|Enum|Equal(Enum) (.Slot (Utilities|Struct|BreakPlayerKeyMapping _array_element_2)) "First") (== (.currentinputaction _array_element) (.AssociatedInputAction (Utilities|Struct|BreakPlayerKeyMapping _array_element_2))))
        (bind _returnvalue_3 (Game|ConstructObjectfromClass InPlayerController "/HumMenuPlugin/Blueprints/OptionsMenuBlueprints/MainObjects/BP_OptionKey.BP_OptionKey_C" self (.CurrentKey (Utilities|Struct|BreakPlayerKeyMapping _array_element_2)) (.MappingName (Utilities|Struct|BreakPlayerKeyMapping _array_element_2)) (.DisplayName (Utilities|Struct|BreakPlayerKeyMapping _array_element_2)) (Utilities|String|StringToName (Utilities|String|ToString(Text) (Utilities|Text|FormatText "key{index}" _array_index)))))
        (Utilities|Array|Add (Variables|Default|GetBlockOptions) _returnvalue_3))))
  (return (Variables|Default|GetBlockOptions)))

(fn RegisterMappingContexts
  (Utilities|Set|Clear (Variables|Default|GetUserMappingsContexts))
  (bind _returnvalue (Class|MenuPluginBlueprintLibrary|GetWidgetPropertiesDataAsset))
  (bind _returnvalue_2 (Utilities|LoadAssetBlocking _returnvalue))
  (bind _aswidgets_properties_data_asset (Utilities|Casting|CastToWidgetsPropertiesDataAsset _returnvalue_2))
  (for _array_element (Variables|/Script/HumMenuPlugin.BindingMappingsDataAsset|GetCurrentMappingContexts (Variables|/Script/HumMenuPlugin.WidgetsPropertiesDataAsset|GetBindingMappings _aswidgets_properties_data_asset))
    (Utilities|Set|Add (Variables|Default|GetUserMappingsContexts) _array_element))
  (bind _returnvalue_3 (Class|EnhancedInputUserSettings|RegisterInputMappingContexts (Class|EnhancedInputSubsystemInterface|GetUserSettings (PlayerController|LocalPlayerSubsystems|GetEnhancedInputLocalPlayerSubsystem (Variables|Default|GetUserPlayerController))) (Variables|Default|GetUserMappingsContexts)))
  (return _returnvalue_3))

(fn GetUserKeyMapping
  (bind _values (Utilities|Map|Values (Class|EnhancedPlayerMappableKeyProfile|GetPlayerMappingRows (Class|EnhancedInputUserSettings|GetCurrentKeyProfile (Class|EnhancedInputSubsystemInterface|GetUserSettings (PlayerController|LocalPlayerSubsystems|GetEnhancedInputLocalPlayerSubsystem (Variables|Default|GetUserPlayerController)))))))
  (Utilities|Array|Clear (Variables|Default|GetUserKeyMapping))
  (for _array_element _values
    (bind _result (Utilities|Set|ToArray (.mappings _array_element)))
    (Utilities|Array|AppendArray (Variables|Default|GetUserKeyMapping) _result)))

(fn CanBindNewKey?
  (params (NewKey :type Key%20Structure :default "None"))
  (CallFunction|GetUserKeyMapping)
  (bind _array_element (Utilities|Array|ForEachLoopwithBreak (Variables|Default|GetUserKeyMapping) :!label _label)
    (:LoopBody
      (if (== NewKey (.CurrentKey (Utilities|Struct|BreakPlayerKeyMapping _array_element)))
        (LocalVariables|SetCanBind false)
        (goto _label Break)
        (else
          (LocalVariables|SetCanBind true))))
    (:Completed
      (return (LocalVariables|GetCanBind) NewKey))))

(fn SetNewKey
  (params (InNewKey :type Key%20Structure :default "None") (MappingName :type Name))
  (Class|EnhancedInputUserSettings|MapPlayerKey (Variables|Default|GetUserSettings) (Utilities|Struct|MakeMapPlayerKeyArgs MappingName "First" InNewKey)))