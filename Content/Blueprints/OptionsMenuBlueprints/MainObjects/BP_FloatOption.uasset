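; BP_FloatOption is an options menu entry for a float setting, shown as a slider.
; Its GetOptionWidget override calls the parent, creates a WB_SliderOption from the option's min, max and current values, and binds to its update event.
; The slider is then passed to CreateOptionWidget, whose result is returned.
; The float update handler only prints the value; this file does not apply or save it.
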(fn GetOptionWidget
  (params (WorldContextObject :type Object%20Object%20Reference) (InPlayerController :type Player%20Controller%20Object%20Reference))
  (|CallParentFunction WorldContextObject InPlayerController)
  (bind _returnvalue (UserInterface|CreateWidget "/HumMenuPlugin/MenuWIdgetElements/OptionsElements/WB_SliderOption.WB_SliderOption_C" InPlayerController (Variables|Default|GetMinVal) (Variables|Default|GetMaxVal) (Variables|Default|GetCurrentValue) WorldContextObject))
  (EventDispatchers|BindEventtoOnFloatOptionUpdate _returnvalue (EventDispatchers|CreateEvent :!event OnFloatOptionUpdatee))
  (bind _returnvalue_2 (Class|OptionObject|CreateOptionWidget WorldContextObject InPlayerController _returnvalue))
  (return _returnvalue_2))

(fn OnFloatOptionUpdatee
  (params (CurrentValue :type Float%20%28double-precision%29))
  (Development|PrintString 0 (Utilities|String|ToString(Float) CurrentValue)))