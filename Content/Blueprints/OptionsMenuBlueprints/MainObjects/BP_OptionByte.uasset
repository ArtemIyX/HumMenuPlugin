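; BP_OptionByte is an options menu entry for a byte value, shown as a selector between named choices.
; GetOptionWidget creates a WB_SelectorOption seeded with the choices, current value and the option itself.
; CreateOptionWidget wraps that selector in a WB_BaseOptonsButton labeled with the option name and returns the button.
; ByteOptionUpdate broadcasts a new value through OnByteOptionUpdate, then stores it as CurrentValue.
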(fn GetOptionWidget
  (params (WorldContextObject :type Object%20Object%20Reference) (InPlayerController :type Player%20Controller%20Object%20Reference))
  (|CallParentFunction WorldContextObject InPlayerController)
  (bind _returnvalue (Class|OptionObject|CreateNewWidget InPlayerController "/HumMenuPlugin/MenuWIdgetElements/OptionsElements/WB_SelectorOption.WB_SelectorOption_C"))
  (bind _aswb_selector_option (Utilities|Casting|CastToWB_SelectorOption _returnvalue))
  (Default|StartWidget _aswb_selector_option (Variables|Default|GetParagraphs) (Variables|Default|GetCurrentValue) self)
  (bind _returnvalue_2 (CallFunction|CreateOptionWidget WorldContextObject InPlayerController _returnvalue))
  (return _returnvalue_2))

(fn CreateOptionWidget
  (params (WorldContextObject :type Object%20Object%20Reference) (InPlayerController :type Player%20Controller%20Object%20Reference) (InputWidget :type User%20Widget%20Object%20Reference))
  (|CallParentFunction WorldContextObject InPlayerController InputWidget)
  (bind _returnvalue (Class|OptionObject|CreateNewWidget InPlayerController "/HumMenuPlugin/MenuWIdgetElements/OptionsElements/WB_BaseOptonsButton.WB_BaseOptonsButton_C"))
  (bind _aswb_base_optons_button (Utilities|Casting|CastToWB_BaseOptonsButton _returnvalue))
  (Default|SetName _aswb_base_optons_button (Variables|Default|GetOptionName))
  (Default|AddWidgetinContainer _aswb_base_optons_button InputWidget)
  (return _aswb_base_optons_button))

(fn ByteOptionUpdate
  (params (Val :type Byte))
  (Class|ByteOptionObject|CallonByteOptionUpdate self Val)
  (Variables|Default|SetCurrentValue Val))