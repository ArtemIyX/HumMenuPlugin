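; BP_OptionFloat is an options-menu object that represents a float setting and builds a slider row for it.
; GetOptionWidget creates a WB_SliderOption, starts it with the current value and a reference to itself, then passes it to CreateOptionWidget.
; CreateOptionWidget wraps the slider in a named WB_BaseOptonsButton container and stores a reference to that container.
; FloatOptionUpdate broadcasts the new value through OnFloatOptionUpdate, then saves it as CurrentValue.
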(fn GetOptionWidget
  (params (WorldContextObject :type Object%20Object%20Reference) (InPlayerController :type Player%20Controller%20Object%20Reference))
  (|CallParentFunction WorldContextObject InPlayerController)
  (bind _returnvalue (Class|OptionObject|CreateNewWidget InPlayerController "/HumMenuPlugin/MenuWIdgetElements/OptionsElements/WB_SliderOption.WB_SliderOption_C"))
  (bind _aswb_slider_option (Utilities|Casting|CastToWB_SliderOption _returnvalue))
  (Default|StartWidget _aswb_slider_option (Variables|Default|GetCurrentValue) 0.0 0.0 self)
  (bind _returnvalue_2 (CallFunction|CreateOptionWidget WorldContextObject InPlayerController _returnvalue))
  (return _returnvalue_2))

(fn CreateOptionWidget
  (params (WorldContextObject :type Object%20Object%20Reference) (InPlayerController :type Player%20Controller%20Object%20Reference) (InputWidget :type User%20Widget%20Object%20Reference))
  (|CallParentFunction WorldContextObject InPlayerController InputWidget)
  (bind _returnvalue (Class|OptionObject|CreateNewWidget InPlayerController "/HumMenuPlugin/MenuWIdgetElements/OptionsElements/WB_BaseOptonsButton.WB_BaseOptonsButton_C"))
  (bind _aswb_base_optons_button (Utilities|Casting|CastToWB_BaseOptonsButton _returnvalue))
  (Default|SetName _aswb_base_optons_button (Variables|Default|GetOptionName))
  (Variables|Default|SetOptionWidgetRef _aswb_base_optons_button)
  (Default|AddWidgetinContainer _aswb_base_optons_button InputWidget)
  (return _aswb_base_optons_button))

(fn FloatOptionUpdate
  (params (Val :type Float%20%28double-precision%29))
  (Class|FloatOptionObject|CallonFloatOptionUpdate self Val)
  (Variables|Default|SetCurrentValue Val))