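; BP_OptionKey is an options-menu option object for rebinding an input key.
; It spawns a key-binding widget showing the current key and wraps it in a named base options button.
; On a key change it fires the update callback, then asks its current block whether the key can bind.
; If allowed, it sets the mapping's key, refreshes the widget and applies Enhanced Input user settings.
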(fn CreateOptionWidget
  (params (WorldContextObject :type Object%20Object%20Reference) (InPlayerController :type Player%20Controller%20Object%20Reference) (InputWidget :type User%20Widget%20Object%20Reference))
  (|CallParentFunction WorldContextObject InPlayerController InputWidget)
  (bind _returnvalue (Class|OptionObject|CreateNewWidget InPlayerController "/HumMenuPlugin/MenuWIdgetElements/OptionsElements/WB_BaseOptonsButton.WB_BaseOptonsButton_C"))
  (bind _aswb_base_optons_button (Utilities|Casting|CastToWB_BaseOptonsButton _returnvalue))
  (Default|SetName _aswb_base_optons_button (Variables|Default|GetOptionName))
  (Default|AddWidgetinContainer _aswb_base_optons_button InputWidget)
  (return _aswb_base_optons_button))

(fn GetOptionWidget
  (params (WorldContextObject :type Object%20Object%20Reference) (InPlayerController :type Player%20Controller%20Object%20Reference))
  (|CallParentFunction WorldContextObject InPlayerController)
  (Variables|Default|SetCurrentController InPlayerController)
  (bind _returnvalue (Class|OptionObject|CreateNewWidget InPlayerController "/HumMenuPlugin/MenuWIdgetElements/OptionsElements/WB_KeyBindingWidget.WB_KeyBindingWidget_C"))
  (bind _aswb_key_binding_widget (Utilities|Casting|CastToWB_KeyBindingWidget _returnvalue))
  (Variables|Default|SetKeyBindingWidgetRef _aswb_key_binding_widget)
  (Default|StartWidget _aswb_key_binding_widget (Variables|Default|GetCurrentKey) self)
  (bind _returnvalue_2 (CallFunction|CreateOptionWidget WorldContextObject InPlayerController _returnvalue))
  (return _returnvalue_2))

(fn KeyOptionUpdate
  (params (NewKey :type Key%20Structure :default "None"))
  (bind _currentblock (Variables|Default|GetCurrentBlock))
  (bind _output_get (Variables|Default|SetCurrentKey NewKey))
  (Class|KeyOptionObject|CallonKeyOptionUpdate self _output_get)
  (Utilities|IsValid _currentblock
    (:Is%20Valid
      (bind (_canbind_ _outnewkey) (Default|CanBindNewKey? _currentblock _output_get))
      (if _canbind_
        (Default|SetNewKey (Variables|Default|GetCurrentBlock) _outnewkey (Variables|Default|GetMappingName))
        (Default|UpdateWidget (Variables|Default|GetKeyBindingWidgetRef) _outnewkey)
        (Class|EnhancedInputUserSettings|ApplySettings (Class|EnhancedInputSubsystemInterface|GetUserSettings (PlayerController|LocalPlayerSubsystems|GetEnhancedInputLocalPlayerSubsystem (Variables|Default|GetCurrentController))))))))