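; BP_OptionsBlock represents one named block of options in the options menu and builds the widget that displays it.
; GetOptionsBlockWidget creates a WB_OptionsBlock, stores it as BlockRef, then passes the option objects from GenerateOptions to AddOptions.
; AddOptions gets each object's widget, prints its name to screen and adds it to the block.
; GenerateOptions only forwards the parent implementation's result.
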(event EventAddOptions
  (params (OptionObjects :type Array%20of%20Option%20Object%20Object%20References) (WorldContextObject :type Object%20Object%20Reference) (InPlayerController :type Player%20Controller%20Object%20Reference))
  (for _array_element OptionObjects
    (bind _returnvalue (Class|OptionObject|GetOptionWidget _array_element WorldContextObject InPlayerController))
    (Development|PrintString 0 (Utilities|GetDisplayName _returnvalue))
    (Default|AddNewOption (Variables|Default|GetBlockRef) _returnvalue)))

(fn GetOptionsBlockWidget
  (params (WorldContextObject :type Object%20Object%20Reference) (InPlayerController :type Player%20Controller%20Object%20Reference))
  (|CallParentFunction WorldContextObject InPlayerController)
  (bind _returnvalue (UserInterface|CreateWidget WorldContextObject "/HumMenuPlugin/MenuWIdgetElements/OptionsElements/WB_OptionsBlock.WB_OptionsBlock_C" InPlayerController (Variables|Default|GetBlockName)))
  (Variables|Default|SetBlockRef _returnvalue)
  (bind _outoptions (CallFunction|GenerateOptions WorldContextObject InPlayerController))
  (Class|OptionsBlockObject|AddOptions _outoptions WorldContextObject InPlayerController)
  (return (Variables|Default|GetBlockRef)))

(fn GenerateOptions
  (params (WorldContextObject :type Object%20Object%20Reference) (InPlayerController :type Player%20Controller%20Object%20Reference))
  (bind _outoptions (|CallParentFunction WorldContextObject InPlayerController))
  (return _outoptions))