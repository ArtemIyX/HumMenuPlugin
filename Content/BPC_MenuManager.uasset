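; HUD-owned component that manages the game's main menu, pause menu and a single message box.
; It creates each menu widget for the owning player, loads its buttons, adds it to the viewport and handles mouse cursor visibility.
; Main menu buttons are blocking-loaded from a widget properties data asset, while pause buttons are passed in.
; CreateMenu switches the active sub-widget, title and back command, with an empty widget meaning the root menu.
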(event EventBeginPlay)

(event EventTick
  (params (DeltaSeconds :type Float%20%28single-precision%29)))

(fn CreateMenu
  (params (WidgetCurrent :type User%20Widget%20Class%20Reference) (TitleText :type Text) (BackCommand :type Menu%20Button%20Command%20Class%20Reference))
  (Utilities|IsValid (Variables|Default|GetMainMenuRef)
    (:Is%20Valid
      (Default|SetCurerntIndex (Variables|Default|GetMainMenuRef) WidgetCurrent TitleText BackCommand))))

(fn CreateMainMenu
  (Variables|Default|SetIsActiveMainMenu? true)
  (bind _ashud (Utilities|Casting|CastToHUD (Components|GetOwner)))
  (bind _returnvalue (UserInterface|CreateWidget (Variables|Default|GetMainMenuClass) (Game|Player|GetOwningPlayerController _ashud)))
  (Variables|Default|SetMainMenuRef _returnvalue)
  (bind _arr (CallFunction|GetMainMenuButtons))
  (Default|LoadButtons (Variables|/HumMenuPlugin/MainMenu/WB_BaseMainMenu.WB_BaseMainMenu_C|GetWB_Main_menu (Variables|Default|GetMainMenuRef)) _arr)
  (CallFunction|CreateMenu)
  (UserInterface|Viewport|AddtoViewport (Variables|Default|GetMainMenuRef) (Variables|Default|GetZOrder))
  (Variables|/Script/Engine.PlayerController|SetbShowMouseCursor (Game|Player|GetOwningPlayerController _ashud) true))

(fn CreatePauseMenu
  (params (PauseMenuButtons :type Generatable%20Buttons%20Data%20Asset%20Object%20Reference))
  (Variables|Default|SetIsPauseMenu? true)
  (bind _ashud (Utilities|Casting|CastToHUD (Components|GetOwner)))
  (bind _returnvalue (UserInterface|CreateWidget (Variables|Default|GetPauseMenuClass) (Game|Player|GetOwningPlayerController _ashud)))
  (Variables|Default|SetMainMenuRef _returnvalue)
  (Default|LoadButtons (Variables|/HumMenuPlugin/MainMenu/WB_BaseMainMenu.WB_BaseMainMenu_C|GetWB_Main_menu (Variables|Default|GetMainMenuRef)) (Variables|/Script/HumMenuPlugin.GeneratableButtonsDataAsset|GetButtonActions PauseMenuButtons))
  (CallFunction|CreateMenu)
  (UserInterface|Viewport|AddtoViewport (Variables|Default|GetMainMenuRef) (Variables|Default|GetZOrder))
  (Variables|/Script/Engine.PlayerController|SetbShowMouseCursor (Game|Player|GetOwningPlayerController _ashud) true))

(fn GetMainMenuButtons
  (bind _returnvalue (Class|MenuPluginBlueprintLibrary|GetWidgetPropertiesDataAsset))
  (bind _returnvalue_2 (Utilities|LoadAssetBlocking _returnvalue))
  (bind _aswidgets_properties_data_asset (Utilities|Casting|CastToWidgetsPropertiesDataAsset _returnvalue_2))
  (Utilities|Array|Clear (LocalVariables|GetButtonActionsArr))
  (for _array_element (Variables|/Script/HumMenuPlugin.WidgetsPropertiesDataAsset|GetButtonActions _aswidgets_properties_data_asset)
    (bind _returnvalue_3 (Utilities|LoadAssetBlocking _array_element))
    (bind _asbutton_action_data_asset (Utilities|Casting|CastToButtonActionDataAsset _returnvalue_3))
    (Utilities|Array|Add (LocalVariables|GetButtonActionsArr) _asbutton_action_data_asset))
  (return (LocalVariables|GetButtonActionsArr)))

(fn RemovePauseMenu
  (if (Variables|Default|GetIsPauseMenu?)
    (Variables|Default|SetIsPauseMenu? false)
    (Class|MenuPluginBlueprintLibrary|ClearObject (Variables|Default|GetMainMenuRef))
    (bind _ashud (Utilities|Casting|CastToHUD (Components|GetOwner)))
    (Variables|/Script/Engine.PlayerController|SetbShowMouseCursor (Game|Player|GetOwningPlayerController _ashud) true)))

(fn RemoveMainMenu
  (if (Variables|Default|GetIsActiveMainMenu?)
    (Class|MenuPluginBlueprintLibrary|ClearObject (Variables|Default|GetMainMenuRef))
    (Variables|Default|SetIsActiveMainMenu? false)
    (bind _ashud (Utilities|Casting|CastToHUD (Components|GetOwner)))
    (Variables|/Script/Engine.PlayerController|SetbShowMouseCursor (Game|Player|GetOwningPlayerController _ashud) false)))

(fn AddMessageBox
  (params (MessageBoxRef :type User%20Widget%20Object%20Reference) (MessageBoxOject :type Message%20Box%20Base%20Object%20Reference))
  (if (not (Variables|Default|GetIsHaveMessageBox?))
    (Variables|Default|SetIsHaveMessageBox? true)
    (Variables|Default|SetMessageBoxWidgetRef MessageBoxRef)
    (Variables|Default|SetMessageBoxObject MessageBoxOject)
    (bind _returnvalue (Class|MenuPluginBlueprintLibrary|GetWidgetPropertiesDataAsset))
    (bind _returnvalue_2 (Utilities|LoadAssetBlocking _returnvalue))
    (bind _aswidgets_properties_data_asset (Utilities|Casting|CastToWidgetsPropertiesDataAsset _returnvalue_2))
    (UserInterface|Viewport|AddtoViewport (Variables|Default|GetMessageBoxWidgetRef) (Variables|/Script/HumMenuPlugin.MessageBoxStyle|GetMessageBoxZOrder (Variables|/Script/HumMenuPlugin.WidgetsPropertiesDataAsset|GetMessageBoxDatAsset _aswidgets_properties_data_asset)))))

(fn RemoveMessageBox
  (bind _messageboxwidgetref (Variables|Default|GetMessageBoxWidgetRef))
  (bind _messageboxobject (Variables|Default|GetMessageBoxObject))
  (if (Variables|Default|GetIsHaveMessageBox?)
    (Utilities|FlowControl|Sequence
      (:then_0
        (Utilities|IsValid _messageboxwidgetref
          (:Is%20Valid
            (Class|MenuPluginBlueprintLibrary|ClearObject _messageboxwidgetref))))
      (:then_1
        (Utilities|IsValid _messageboxobject
          (:Is%20Valid
            (Class|MenuPluginBlueprintLibrary|ClearObject _messageboxobject))))
      (:then_2
        (Variables|Default|SetIsHaveMessageBox? false)))))